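; Paper2D side-scroller player character with Mario-style controls, health, and win and game-over screens.
; Enhanced Input drives jumping with a sound and movement along world X, flipping control yaw to face the travel direction.
; Tick swaps between walk and stand flipbooks based on velocity.
; Damage reduces health; reaching zero or a GameWin event shows the matching widget, enables the cursor and pauses the game.
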(event Custom|GameWin
  (bind _returnvalue (UserInterface|CreateWidget "/Game/Blueprints/UI/BP_GameWIN.BP_GameWIN_C" (Game|GetPlayerController 0)))
  (UserInterface|Viewport|AddtoPlayerScreen _returnvalue)
  (Variables|/Script/Engine.PlayerController|SetbShowMouseCursor (Game|GetPlayerController 0) true)
  (Game|SetGamePaused true))

(event Custom|OnReachedJumpApex_Event
  ;[0.15 0.15 0.15 0.5] Movement
)

(event Input|EnhancedActionEvents|EnhancedInputActionIA_Jump
  (params (ActionValue :type Boolean) (ElapsedSeconds :type Float%20%28double-precision%29) (TriggeredSeconds :type Float%20%28double-precision%29) (InputAction :type Input%20Action%20Object%20Reference :default "/Game/Blueprints/Input/Actions/IA_Jump.IA_Jump"))
  ;[0.15 0.15 0.15 0.5] Movement
  (:Started
    (Character|Jump)
    (EventDispatchers|AssignOnReachedJumpApex (delegate Custom|OnReachedJumpApex_Event))
    (Audio|SpawnSoundatLocation "/Game/Music/Jump_or_enemy_hitsound.Jump_or_enemy_hitsound" (Transformation|GetActorLocation) "0, 0, 0" 1.0 1.0 0.0 0 0))
  (:Completed
    (Character|StopJumping)))

(event Input|EnhancedActionEvents|EnhancedInputActionIA_Move
  (params (ActionValue :type Float%20%28double-precision%29) (ElapsedSeconds :type Float%20%28double-precision%29) (TriggeredSeconds :type Float%20%28double-precision%29) (InputAction :type Input%20Action%20Object%20Reference :default "/Game/Blueprints/Input/Actions/IA_Move.IA_Move"))
  ;[0.15 0.15 0.15 0.5] Movement
  (Pawn|Input|AddMovementInput "1.000000,0.000000,0.000000" ActionValue false)
  (Pawn|SetControlRotation (Pawn|GetController) (select (> ActionValue 0.0) (Math|Rotator|MakeRotator 0.0 0.0 0.0) (Math|Rotator|MakeRotator 0.0 0.0 1.8e+02))))

(event EventBeginPlay
  ;[0.15 0.15 0.15 0.5] Basic
  (bind _asplayer_controller (Utilities|Casting|CastToPlayerController (Pawn|GetController)))
  (Input|AddMappingContext (PlayerController|LocalPlayerSubsystems|GetEnhancedInputLocalPlayerSubsystem _asplayer_controller) "/Game/Blueprints/Input/IMC_Mario.IMC_Mario" 0 "(bIgnoreAllPressedKeysUntilRelease=True,bForceImmediately=False,bNotifyUserSettings=False)"))

(event EventTick
  (params (DeltaSeconds :type Float%20%28single-precision%29))
  (if (> (Math|Vector|VectorLength (Transformation|GetVelocity)) 0.0)
    (Sprite|SetFlipbook (Variables|Default|GetSprite) "/Game/PaperAssets/Flipbooks/PC_Walk.PC_Walk")
    (else
      (Sprite|SetFlipbook (Variables|Default|GetSprite) "/Game/PaperAssets/Flipbooks/PC_Stand_Flipbook.PC_Stand_Flipbook"))))

(event Game|Damage|EventAnyDamage
  (params (Damage :type Float%20%28single-precision%29) (DamageType :type Damage%20Type%20Object%20Reference) (InstigatedBy :type Controller%20Object%20Reference) (DamageCauser :type Actor%20Object%20Reference))
  ;[0.15 0.15 0.15 0.5] Damage System
  (Variables|Default|SetHealth (- (Variables|Default|GetHealth) Damage))
  (if (<= (Variables|Default|GetHealth) 0.0)
    ;[0.15 0.15 0.15 0.5] Game Over
    (bind _returnvalue (UserInterface|CreateWidget "/Game/Blueprints/UI/BP_GameOVER.BP_GameOVER_C" (Game|GetPlayerController 0)))
    (UserInterface|Viewport|AddtoPlayerScreen _returnvalue)
    (Variables|/Script/Engine.PlayerController|SetbShowMouseCursor (Game|GetPlayerController 0) true)
    (Game|SetGamePaused true)))

(fn ConstructionScript)