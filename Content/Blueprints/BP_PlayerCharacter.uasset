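; Player character Blueprint that handles movement input, apparently for a Galaga-style game.
; On BeginPlay it waits briefly, then adds the IMC_Galaga mapping context to player 0's Enhanced Input subsystem.
; IA_Move feeds its action value into movement along up and right vectors, derived from actor pitch and roll respectively.
; Each move event also prints a "Hello" debug string.
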(event Input|EnhancedActionEvents|EnhancedInputActionIA_Move
  (params (ActionValue :type Float%20%28double-precision%29) (ElapsedSeconds :type Float%20%28double-precision%29) (TriggeredSeconds :type Float%20%28double-precision%29) (InputAction :type Input%20Action%20Object%20Reference :default "/Game/Blueprints/Input/Actions/IA_Move.IA_Move"))
  (Pawn|Input|AddMovementInput (Math|Vector|GetUpVector (Math|Rotator|MakeRotator 0.0 (.pitch (Transformation|GetActorRotation)) 0.0)) ActionValue false)
  (Pawn|Input|AddMovementInput (Math|Vector|GetRightVector (Math|Rotator|MakeRotator (.roll (Transformation|GetActorRotation)) 0.0 0.0)) ActionValue false)
  (Development|PrintString "Hello"))

(event EventBeginPlay
  (Utilities|FlowControl|Delay 0.2)
  (Input|AddMappingContext (PlayerController|LocalPlayerSubsystems|GetEnhancedInputLocalPlayerSubsystem (Game|GetPlayerController 0)) "/Game/Blueprints/Input/IMC_Galaga.IMC_Galaga" 0 "(bIgnoreAllPressedKeysUntilRelease=True,bForceImmediately=False,bNotifyUserSettings=False)"))

(fn ConstructionScript)