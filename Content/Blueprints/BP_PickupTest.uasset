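; BP_PickupTest is a test pickup, with a mushroom component, that homes toward the player when they come within its Magnet volume.
; Magnet overlaps set or clear the target and a timer, while Tick moves the actor along the normalized direction at Speed, applied as a local offset.
; Any Collision overlap flags it collected, then after a delay destroys the mushroom and collision components.
; Pickup only casts to BP_PlayerTest, with no further effect.
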(event OnComponentBeginOverlap(Magnet)
  (params (OverlappedComponent :type Primitive%20Component%20Object%20Reference) (OtherActor :type Actor%20Object%20Reference) (OtherComp :type Primitive%20Component%20Object%20Reference) (OtherBodyIndex :type Integer) (bFromSweep :type Boolean) (SweepResult :type Hit%20Result%20Structure%20%28by%20ref%29))
  (if (== OtherActor (Game|Player|GetPlayerPawn 0))
    (Variables|Default|SetOther%20Actor OtherActor)
    (bind _returnvalue (Utilities|Time|SetTimerbyEvent (EventDispatchers|CreateEvent :!event Custom|PullTowardsTarget) 0.0))
    (Variables|Default|SetTimer _returnvalue)))

(event OnComponentEndOverlap(Magnet)
  (params (OverlappedComponent :type Primitive%20Component%20Object%20Reference) (OtherActor :type Actor%20Object%20Reference) (OtherComp :type Primitive%20Component%20Object%20Reference) (OtherBodyIndex :type Integer))
  (if (== OtherActor (Game|Player|GetPlayerPawn 0))
    (Variables|Default|SetOther%20Actor 0)
    (Utilities|Time|ClearandInvalidateTimerbyHandle (Variables|Default|GetTimer))))

(event OnComponentBeginOverlap(Collision)
  (params (OverlappedComponent :type Primitive%20Component%20Object%20Reference) (OtherActor :type Actor%20Object%20Reference) (OtherComp :type Primitive%20Component%20Object%20Reference) (OtherBodyIndex :type Integer) (bFromSweep :type Boolean) (SweepResult :type Hit%20Result%20Structure%20%28by%20ref%29))
  (Variables|Default|SetIsCollected? true)
  (Utilities|FlowControl|Delay 2.0)
  (Components|DestroyComponent (Variables|Default|GetMushroom))
  (CallFunction|Pickup))

(event Custom|PullTowardsTarget
  (Transformation|AddActorLocalOffset (* (Math|Vector|Normalize (- (Transformation|GetActorLocation (Variables|Default|GetOther%20Actor)) (Transformation|GetActorLocation))) (Utilities|Time|GetWorldDeltaSeconds) (Variables|Default|GetSpeed)) false false))

(event Custom|Pickup
  (Utilities|Casting|CastToBP_PlayerTest (Game|GetPlayerCharacter 0)))

(event EventTick
  (params (DeltaSeconds :type Float%20%28single-precision%29))
  (Variables|Default|GetOther%20Actor
    (:then
      (CallFunction|PullTowardsTarget))
    (:else)))

(fn ConstructionScript)