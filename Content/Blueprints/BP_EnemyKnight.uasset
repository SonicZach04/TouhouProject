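; BP_EnemyKnight is a patrolling enemy character that damages what it bumps into and is destroyed when its head is hit.
; Tick runs Patrol, driving movement along world X by the MovingRight flag, while the yaw selection resolves to zero either way.
; Capsule hits flip MovingRight and apply fixed damage to the other actor.
; DamageBox hits apply BaseDamage only to BP_PlayerTest, and any HeadCollision hit destroys the knight.
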(event OnComponentHit(CapsuleComponent)
  (params (HitComponent :type Primitive%20Component%20Object%20Reference) (OtherActor :type Actor%20Object%20Reference) (OtherComp :type Primitive%20Component%20Object%20Reference) (NormalImpulse :type Vector :default "0, 0, 0") (Hit :type Hit%20Result%20Structure%20%28by%20ref%29))
  (Variables|Default|SetMoving%20Right (not (Variables|Default|GetMoving%20Right)))
  (Game|Damage|ApplyDamage OtherActor 1e+02 0 0 "/Script/Engine.DamageType"))

(event OnComponentHit(DamageBox)
  (params (HitComponent :type Primitive%20Component%20Object%20Reference) (OtherActor :type Actor%20Object%20Reference) (OtherComp :type Primitive%20Component%20Object%20Reference) (NormalImpulse :type Vector :default "0, 0, 0") (Hit :type Hit%20Result%20Structure%20%28by%20ref%29))
  (bind _asbp_player_test (Utilities|Casting|CastToBP_PlayerTest OtherActor))
  (Game|Damage|ApplyDamage _asbp_player_test (Variables|Default|GetBase%20Damage) 0 self "/Script/Engine.DamageType"))

(event OnComponentHit(HeadCollision)
  (params (HitComponent :type Primitive%20Component%20Object%20Reference) (OtherActor :type Actor%20Object%20Reference) (OtherComp :type Primitive%20Component%20Object%20Reference) (NormalImpulse :type Vector :default "0, 0, 0") (Hit :type Hit%20Result%20Structure%20%28by%20ref%29))
  (Actor|DestroyActor))

(event Custom|Patrol
  (Transformation|SetRelativeRotation (Variables|Collision|GetCapsuleComponent) (Math|Rotator|MakeRotator 0.0 0.0 (Math|Float|SelectFloat 0.0 0.0 (Variables|Default|GetMoving%20Right))) false false)
  (Pawn|Input|AddMovementInput (Math|Vector|SelectVector "1.000000,0.000000,0.000000" "-1.000000,0.000000,0.000000" (Variables|Default|GetMoving%20Right)) 1.0 false))

(event EventBeginPlay)

(event Collision|EventActorBeginOverlap
  (params (OtherActor :type Actor%20Object%20Reference)))

(event EventTick
  (params (DeltaSeconds :type Float%20%28single-precision%29))
  (CallFunction|Patrol))

(fn ConstructionScript)