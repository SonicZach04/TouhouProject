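; Behavior tree task that drives a flying AI character by setting its movement velocity directly.
; On execute it casts the controlled pawn to Character and sets CharacterMovement velocity to PatrolLocationAI at index 2, scaled by Speed.
; The patrol value is used as is, without subtracting the pawn's position or normalizing, and the task finishes successfully right away.
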(event EventReceiveExecuteAI
  (params (OwnerController :type AI%20Controller%20Object%20Reference) (ControlledPawn :type Pawn%20Object%20Reference))
  (bind _output_get (Variables|Default|SetControlled%20Pawn ControlledPawn))
  (bind _ascharacter (Utilities|Casting|CastToCharacter _output_get))
  (Variables|Default|SetCharacter%20Movement (Variables|/Script/Engine.Character|GetCharacterMovement _ascharacter))
  (Variables|/Script/Engine.MovementComponent|SetVelocity (Variables|Default|GetCharacter%20Movement) (* (Utilities|Array|Get(acopy) (Variables|Default|GetPatrolLocationAI) 2) (Variables|Default|GetSpeed)))
  (AI|BehaviorTree|FinishExecute true))