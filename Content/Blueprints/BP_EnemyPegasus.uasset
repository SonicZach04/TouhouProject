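; BP_EnemyPegasus is a flying enemy that patrols along the world X axis, reversing direction and damaging whatever its capsule hits.
; Tick drives both movement and shooting, with a two-second Delay throttling BP_Bullet spawns just below the Pegasus.
; Any hit on HeadBox destroys it, while any hit on DamageBox damages the BP_PlayerTest player, regardless of what made contact.
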(event OnComponentHit(CapsuleComponent)
  (params (HitComponent :type Primitive%20Component%20Object%20Reference) (OtherActor :type Actor%20Object%20Reference) (OtherComp :type Primitive%20Component%20Object%20Reference) (NormalImpulse :type Vector :default "0, 0, 0") (Hit :type Hit%20Result%20Structure%20%28by%20ref%29))
  (Variables|Default|SetMoving%20Right (not (Variables|Default|GetMoving%20Right)))
  (Game|Damage|ApplyDamage OtherActor (Variables|Default|GetBase%20Damage) 0 0))

(event OnComponentHit(HeadBox)
  (params (HitComponent :type Primitive%20Component%20Object%20Reference) (OtherActor :type Actor%20Object%20Reference) (OtherComp :type Primitive%20Component%20Object%20Reference) (NormalImpulse :type Vector :default "0, 0, 0") (Hit :type Hit%20Result%20Structure%20%28by%20ref%29))
  (Actor|DestroyActor))

(event OnComponentHit(DamageBox)
  (params (HitComponent :type Primitive%20Component%20Object%20Reference) (OtherActor :type Actor%20Object%20Reference) (OtherComp :type Primitive%20Component%20Object%20Reference) (NormalImpulse :type Vector :default "0, 0, 0") (Hit :type Hit%20Result%20Structure%20%28by%20ref%29))
  (bind _asbp_player_test (Utilities|Casting|CastToBP_PlayerTest (Game|GetPlayerCharacter 0)))
  (Game|Damage|ApplyDamage _asbp_player_test (Variables|Default|GetBase%20Damage) 0 0 "/Script/Engine.DamageType"))

(event Custom|Patrol
  (Transformation|SetRelativeRotation (Variables|Collision|GetCapsuleComponent) (Math|Rotator|MakeRotator 0.0 0.0 (Math|Float|SelectFloat 0.0 1.8e+02 (Variables|Default|GetMoving%20Right))) false false)
  (Pawn|Input|AddMovementInput (Math|Vector|SelectVector "1.000000,0.000000,0.000000" "-1.000000,0.000000,0.000000" (Variables|Default|GetMoving%20Right)) 1.0 false))

(event Custom|BulletHell
  ;[0.15 0.15 0.15 0.5] Bullet
  (Utilities|FlowControl|Delay 2.0)
  (Game|SpawnActorfromClass "/Game/Blueprints/BP_Bullet.BP_Bullet_C" (Math|Conversions|ToTransform(Vector) (Math|Transform|TransformLocation (Transformation|GetActorTransform (Components|GetOwner (Variables|Default|GetPegasus))) "0.000000,0.000000,-3.000000")) "Undefined" "MultiplyWithRoot" 0 0))

(event EventBeginPlay
  (Pawn|Components|CharacterMovement|SetMovementMode (Variables|Character|GetCharacterMovement) "MOVE_Flying" 0))

(event EventTick
  (params (DeltaSeconds :type Float%20%28single-precision%29))
  (CallFunction|Patrol)
  (CallFunction|BulletHell))

(fn ConstructionScript)